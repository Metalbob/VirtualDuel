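; Receptacle Blueprint that serves as a team-colored drop-off point for stealable items.
; On BeginPlay it sets the Base material to red or blue according to ColorToReceive.
; When a StealableItem_BP with a matching team color overlaps the Box, it detaches the item, disables its physics, teleports it to the Sphere's location and activates a particle effect.
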(event OnComponentBeginOverlap(Box)
  (params (OverlappedComponent :type Primitive%20Component%20Object%20Reference) (OtherActor :type Actor%20Object%20Reference) (OtherComp :type Primitive%20Component%20Object%20Reference) (OtherBodyIndex :type Integer) (bFromSweep :type Boolean) (SweepResult :type Hit%20Result%20Structure%20%28by%20ref%29))
  (bind _asstealable_item_bp (Utilities|Casting|CastToStealableItem_BP OtherActor))
  (if (Utilities|Enum|Equal(Enum) (Variables|/Script/VirtualDuel.StealableItem|GetteamColor _asstealable_item_bp) (Variables|Default|GetcolorToReceive))
    (Transformation|DetachFromActor OtherActor "KeepRelative" "KeepRelative" "KeepRelative")
    (Physics|SetSimulatePhysics (Variables|/Script/Engine.StaticMeshActor|GetStaticMeshComponent _asstealable_item_bp) false)
    (Transformation|SetActorLocation OtherActor (Transformation|GetWorldLocation (Variables|Default|GetSphere)) false true)
    (Components|Activation|Activate (Variables|Default|GetParticleSystem) false)))

(event EventBeginPlay
  (switch Utilities|FlowControl|Switch|SwitchonETeam (Variables|Default|GetcolorToReceive)
    (:RED
      (Rendering|Material|SetMaterial (Variables|Default|GetBase) 0 "/Game/Materials/Red.Red"))
    (:BLUE
      (Rendering|Material|SetMaterial (Variables|Default|GetBase) 0 "/Game/Materials/Blue.Blue"))))

(event Collision|EventActorBeginOverlap
  (params (OtherActor :type Actor%20Object%20Reference)))

(event EventTick
  (params (DeltaSeconds :type Float%20%28single-precision%29)))

(fn ConstructionScript)