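; StealableItem_BP is a team-colored item actor that can be picked up and dropped.
; On BeginPlay it sets the static mesh material to red or blue from TeamColor.
; Pickup, gated by the Grababble flag, disables mesh physics and attaches the root component to the supplied component, keeping world transform.
; Drop re-enables physics and detaches the actor in place.
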(event EventBeginPlay
  (switch Utilities|FlowControl|Switch|SwitchonETeam (Variables|Default|GetteamColor)
    (:RED
      (Rendering|Material|SetMaterial (Variables|Default|GetStaticMeshComponent) 0 "/Game/Materials/Red.Red"))
    (:BLUE
      (Rendering|Material|SetMaterial (Variables|Default|GetStaticMeshComponent) 0 "/Game/Materials/Blue.Blue"))))

(event Collision|EventActorBeginOverlap
  (params (OtherActor :type Actor%20Object%20Reference)))

(event EventTick
  (params (DeltaSeconds :type Float%20%28single-precision%29)))

(event EventPickup
  (params (AttachTo :type Scene%20Component%20Object%20Reference))
  (if (Variables|Default|Getgrababble)
    (Physics|SetSimulatePhysics (Variables|Default|GetStaticMeshComponent) false)
    (Transformation|AttachComponentToComponent (VehicleSound|GetRootComponent) AttachTo "None" "KeepWorld" "KeepWorld" "KeepWorld" false)))

(event EventDrop
  (Physics|SetSimulatePhysics (Variables|Default|GetStaticMeshComponent) true)
  (Transformation|DetachFromActor "KeepWorld" "KeepWorld" "KeepWorld"))

(fn ConstructionScript)